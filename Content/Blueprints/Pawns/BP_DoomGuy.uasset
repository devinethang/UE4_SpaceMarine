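; BP_DoomGuy is the player pawn, with world-axis movement and mouse-driven yaw aiming independent of movement.
; Forward and right input axes feed movement input directly.
; Each tick, mouse velocity above a deadzone becomes a yaw via Atan2, and control rotation eases toward it with RInterpTo smoothing.
; An unconnected thumbstick aim branch never runs, and its deadzone check mixes aim-up with move-right input.
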(event `InputAxis|MoveForward`
  (params (AxisValue :type "Float (single-precision)"))
  (`self.AddMovementInput` (1.0 0.0 0.0) AxisValue))

(event `InputAxis|MoveRight`
  (params (AxisValue :type "Float (single-precision)"))
  (`self.AddMovementInput` (0.0 1.0 0.0) AxisValue))

(event `self.ReceiveTick`
  (params (DeltaSeconds :type "Float (single-precision)"))
  (`self.Update  Player Aim`))

(fn `Get Mouse Velocity `
  (returns (ReturnValue :type "Vector2D Structure"))
  (bind (_deltax _deltay) (`PlayerController.GetInputMouseDelta` (`GameplayStatics.GetPlayerController` 0)))
  (return (/ (`KismetMathLibrary.MakeVector2D` _deltax _deltay) (`GameplayStatics.GetWorldDeltaSeconds`))))

(fn `Is Mouse Above Deadzone`
  (returns (ReturnValue :type Boolean))
  (bind _returnvalue (`self.Get Mouse Velocity `))
  (return (> (`KismetMathLibrary.VSize2D` _returnvalue) (`self.Mouse Deadzone`))))

(fn `Is thumbstick above dead zone`
  (returns (ReturnValue :type Boolean))
  (return (> (`KismetMathLibrary.VSize2D` (`KismetMathLibrary.MakeVector2D` (`self.GetInputAxisValue`) (`self.GetInputAxisValue`))) (`self.Thumbstick Deadzone`))))

(fn `Update  Player Aim`
  (bind _returnvalue (`GameplayStatics.GetPlayerController` 0))
  (bind _returnvalue_2 (`self.Is Mouse Above Deadzone`))
  (if _returnvalue_2
    (bind _returnvalue_3 (`self.Get Mouse Velocity `))
    (`Controller.SetControlRotation` _returnvalue (`KismetMathLibrary.RInterpTo` (`Controller.GetControlRotation` _returnvalue) (`KismetMathLibrary.MakeRotator` 0.0 0.0 (`KismetMathLibrary.DegAtan2` (`KismetMathLibrary.BreakVector2D` _returnvalue_3) (`.Y` (`KismetMathLibrary.BreakVector2D` _returnvalue_3)))) (`GameplayStatics.GetWorldDeltaSeconds`) (`self.Mouse Smoothing Strength`)))))

(fn `UserConstructionScript`)